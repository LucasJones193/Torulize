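; BP_Exit is a level exit that completes the level when the player stays inside it for TimeToExit seconds.
; Overlap starts a door timer and a camera fade with audio; leaving early stops both.
; When Tick's timer expires, it marks DoorID completed and commits this run's collected bonuses in the game instance, then opens MainMenu.
; BeginPlay clears that pending bonus list, so only bonuses from a finished run are saved.
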(event EventBeginPlay
  (bind _asgi_game_instance (Utilities|Casting|CastToGI_GameInstance (Game|GetGameInstance)))
  (Variables|Default|SetGame%20Instance _asgi_game_instance)
  (Utilities|Array|Clear (Variables|/Game/Collectables/GI_GameInstance.GI_GameInstance_C|GetCurrently%20Collected%20Bonuses%20 (Variables|Default|GetGame%20Instance))))

(event Collision|EventActorBeginOverlap
  (params (OtherActor :type Actor%20Object%20Reference))
  (if (== (Utilities|GetClass OtherActor) "/Game/Player/CBP_Player.CBP_Player_C")
    (Variables|Default|SetOnDoor true)
    (Variables|Default|SetDoorTime 0.0)
    (CameraFades|StartCameraFade :self (Game|GetPlayerCameraManager 0) :ToAlpha 1.0 :Duration (Variables|Default|GetTimeToExit) :bShouldFadeAudio true :bHoldWhenFinished true)))

(event EventTick
  (params (DeltaSeconds :type Float%20%28single-precision%29))
  (bind _game_instance (Variables|Default|GetGame%20Instance))
  (if (Variables|Default|GetOnDoor)
    (bind _output_get (Variables|Default|SetDoorTime (+ DeltaSeconds (Variables|Default|GetDoorTime))))
    (if (>= _output_get (Variables|Default|GetTimeToExit))
      (Utilities|Array|SetArrayElem (Variables|/Game/Collectables/GI_GameInstance.GI_GameInstance_C|GetCompletedLevels _game_instance) (Variables|Default|GetDoorID) true)
      (for _array_element (Variables|/Game/Collectables/GI_GameInstance.GI_GameInstance_C|GetCurrently%20Collected%20Bonuses%20 _game_instance)
        (Utilities|Array|SetArrayElem (Variables|/Game/Collectables/GI_GameInstance.GI_GameInstance_C|GetCollected%20Bonuses _game_instance) _array_element true true))
      (Utilities|Array|Clear (Variables|/Game/Collectables/GI_GameInstance.GI_GameInstance_C|GetCurrently%20Collected%20Bonuses%20 (Variables|Default|GetGame%20Instance)))
      (Game|OpenLevel(byName) "MainMenu"))))

(event Collision|EventActorEndOverlap
  (params (OtherActor :type Actor%20Object%20Reference))
  (if (== (Utilities|GetClass OtherActor) "/Game/Player/CBP_Player.CBP_Player_C")
    (Variables|Default|SetOnDoor false)
    (CameraFades|StopCameraFade (Game|GetPlayerCameraManager 0))))

(fn ConstructionScript)