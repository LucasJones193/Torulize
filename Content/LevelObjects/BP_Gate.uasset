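; BP_Gate is a level-object gate that opens and closes by scaling its Hinge component along the Z axis.
; A timeline's OpenTack track drives that scale, playing forward on Open and in reverse on Close.
; SwitchState toggles the State boolean and calls the matching event, and BeginPlay applies the initial State the same way.
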(event Custom|Open
  (bind _open_tack (Timeline|Timeline Play)
    (:Update
      (Transformation|SetRelativeScale3D (Variables|Default|GetHinge) (Math|Vector|MakeVector 1.0 1.0 _open_tack)))))

(event Custom|Close
  (bind _open_tack (Timeline|Timeline Reverse)
    (:Update
      (Transformation|SetRelativeScale3D (Variables|Default|GetHinge) (Math|Vector|MakeVector 1.0 1.0 _open_tack)))))

(event EventSwitchState
  (bind _output_get (Variables|Default|SetState (not (Variables|Default|GetState))))
  (if _output_get
    (CallFunction|Open)
    (else
      (CallFunction|Close))))

(event EventBeginPlay
  (if (Variables|Default|GetState)
    (CallFunction|Open)
    (else
      (CallFunction|Close))))

(fn ConstructionScript)