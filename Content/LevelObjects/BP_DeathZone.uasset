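; Switchable death zone that fades the screen to near-black and reloads the current level when the player stays inside it.
; Overlap while on plays a fade timeline on the camera manager, and leaving reverses it, so reload only happens if the fade finishes at full.
; SwitchState toggles the zone and plays or reverses a timeline that scales its X and Z between the starting scale and a fixed size.
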(event Collision|EventActorBeginOverlap
  (params (OtherActor :type Actor%20Object%20Reference))
  (if (and (== (Utilities|GetClass OtherActor) "/Game/Player/CBP_Player.CBP_Player_C") (Variables|Default|GetOn))
    (bind _fade (Timeline|FadeOut Play)
      (:Update
        (Class|PlayerCameraManager|SetManualCameraFade (Game|GetPlayerCameraManager 0) _fade "(R=0.000000,G=0.010330,B=0.000000,A=1.000000)" false))
      (:Finished
        (if (>= _fade 1.5)
          (bind _returnvalue (Game|GetCurrentLevelName true))
          (Game|OpenLevel(byName) (Utilities|String|StringToName _returnvalue)))))))

(event Collision|EventActorEndOverlap
  (params (OtherActor :type Actor%20Object%20Reference))
  (if (== (Utilities|GetClass OtherActor) "/Game/Player/CBP_Player.CBP_Player_C")
    (bind _fade (Timeline|FadeOut Reverse)
      (:Update
        (Class|PlayerCameraManager|SetManualCameraFade (Game|GetPlayerCameraManager 0) _fade "(R=0.000000,G=0.010330,B=0.000000,A=1.000000)" false))
      (:Finished
        (if (>= _fade 1.5)
          (bind _returnvalue (Game|GetCurrentLevelName true))
          (Game|OpenLevel(byName) (Utilities|String|StringToName _returnvalue)))))))

(event EventSwitchState
  (Variables|Default|SetOn (not (Variables|Default|GetOn)))
  (if (Variables|Default|GetOn)
    (bind _newtrack_0 (Timeline|Grow/Shrink Play)
      (:Update
        (Transformation|SetActorScale3D (Math|Vector|MakeVector (Math|Float|Lerp (.x (Variables|Default|GetBeginScale)) 4.0 _newtrack_0) 0.5 (Math|Float|Lerp (.z (Variables|Default|GetBeginScale)) 4.0 _newtrack_0)))))
    (else
      (Timeline|Grow/Shrink Reverse))))

(event EventBeginPlay
  (Variables|Default|SetBeginScale (Transformation|GetActorScale3D))
  (if (not (Variables|Default|GetOn))
    (Transformation|SetActorScale3D "4.000000,4.000000,1.000000")))

(fn ConstructionScript)