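; Two-position lever that the player pushes by walking through it, toggling the linked gates.
; Overlap begin and end compare the player's X position to the lever's, tilting the hinge in the direction of travel.
; LeftOn sets which side counts as on, and each change in that state calls SwitchState on every gate in GateReference.
; BeginPlay sets the starting tilt, state and platform material.
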(event Custom|TestForOpeness
  (if (!= (== (Variables|Default|GetLeftOn) (Variables|Default|GetLeft)) (Variables|Default|GetState))
    (Variables|Default|SetState (not (Variables|Default|GetState)))
    (for _array_element (Variables|Default|GetGateReference)
      (Default|SwitchState _array_element))))

(event EventBeginPlay
  (Utilities|FlowControl|Sequence
    (:then_0
      (if (Variables|Default|GetLeft)
        (Transformation|SetRelativeRotation (Variables|Default|GetHinge) "30.000000,0.000000,0.000000" false false)
        (else
          (Transformation|SetRelativeRotation (Variables|Default|GetHinge) "-30.000000,0.000000,0.000000" false false))))
    (:then_1
      (Variables|Default|SetState (== (Variables|Default|GetLeftOn) (Variables|Default|GetLeft)))
      (CallFunction|TestforOpeness))
    (:then_2
      (Rendering|Material|SetMaterial (Variables|Default|GetPlatform) 0 (Variables|Default|GetMaterial)))))

(event Collision|EventActorBeginOverlap
  (params (OtherActor :type Actor%20Object%20Reference))
  (if (== (Utilities|GetClass OtherActor) "/Game/Player/CBP_Player.CBP_Player_C")
    (if (< (- (.x (Transformation|GetActorLocation OtherActor)) (.x (Transformation|GetActorLocation))) 0.0)
      (Variables|Default|SetLeft false)
      (Transformation|SetRelativeRotation (Variables|Default|GetHinge) "-30.000000,0.000000,0.000000" false false)
      (else
        (Variables|Default|SetLeft true)
        (Transformation|SetRelativeRotation (Variables|Default|GetHinge) "30.000000,0.000000,0.000000" false false)))
    (CallFunction|TestforOpeness)))

(event Collision|EventActorEndOverlap
  (params (OtherActor :type Actor%20Object%20Reference))
  (if (== (Utilities|GetClass OtherActor) "/Game/Player/CBP_Player.CBP_Player_C")
    (if (< (- (.x (Transformation|GetActorLocation OtherActor)) (.x (Transformation|GetActorLocation))) 0.0)
      (Variables|Default|SetLeft true)
      (Transformation|SetRelativeRotation (Variables|Default|GetHinge) "30.000000,0.000000,0.000000" false false)
      (else
        (Variables|Default|SetLeft false)
        (Transformation|SetRelativeRotation (Variables|Default|GetHinge) "-30.000000,0.000000,0.000000" false false)))
    (CallFunction|TestforOpeness)))

(fn ConstructionScript)