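; BP_Bonus is a collectable pickup, identified by its Bonus variable, that the player picks up by overlapping it.
; On BeginPlay it caches GI_GameInstance and destroys itself if CollectedBonuses already marks its Bonus as collected.
; An overlap by an actor of exactly CBP_Player class adds the Bonus to CurrentlyCollectedBonuses, a separate collection from the one checked at start, then destroys the pickup.
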(event EventBeginPlay
  (bind _asgi_game_instance (Utilities|Casting|CastToGI_GameInstance (Game|GetGameInstance)))
  (Variables|Default|SetGame%20Instance _asgi_game_instance)
  (if (Utilities|Array|Get(acopy) (Variables|/Game/Collectables/GI_GameInstance.GI_GameInstance_C|GetCollected%20Bonuses _asgi_game_instance) (Variables|Default|GetBonus#))
    (Actor|DestroyActor)))

(event Collision|EventActorBeginOverlap
  (params (OtherActor :type Actor%20Object%20Reference))
  (if (== (Utilities|GetClass OtherActor) "/Game/Player/CBP_Player.CBP_Player_C")
    (Utilities|Array|Add (Variables|/Game/Collectables/GI_GameInstance.GI_GameInstance_C|GetCurrently%20Collected%20Bonuses%20 (Variables|Default|GetGame%20Instance)) (Variables|Default|GetBonus#))
    (Actor|DestroyActor)))

(fn ConstructionScript)